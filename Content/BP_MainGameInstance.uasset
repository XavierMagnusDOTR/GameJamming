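; Game instance that centralizes level travel and screen switching between the main menu, gameplay HUD, escape menu and victory/death menu.
; StartNewGame and LoadMainMenu open their level and immediately create their widget, with only the HUD reference stored.
; InitializeMainMenu and the other menu functions add UI in the current level with UI-only input.
; ResumeGame restores game-only input and hides the cursor, without removing any widget.
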(fn StartNewGame
  (bind _returnvalue (Game|GetPlayerController 0))
  (Game|OpenLevel(byObjectReference) "/Game/TestingZone.TestingZone")
  (bind _returnvalue_2 (UserInterface|CreateWidget "/Game/UI/WBP_GameHUD.WBP_GameHUD_C" _returnvalue))
  (UserInterface|Viewport|AddtoViewport _returnvalue_2 0)
  (Input|SetInputModeGameandUI _returnvalue _returnvalue_2 "DoNotLock" true)
  (Variables|Default|SetRefGameHUD _returnvalue_2))

(fn LoadMainMenu
  (bind _returnvalue (Game|GetPlayerController 0))
  (Game|OpenLevel(byObjectReference) "/Game/MainMenu.MainMenu")
  (bind _returnvalue_2 (UserInterface|CreateWidget "/Game/UI/WBP_MainMenu.WBP_MainMenu_C" _returnvalue))
  (UserInterface|Viewport|AddtoViewport _returnvalue_2 0)
  (Input|SetInputModeUIOnly _returnvalue _returnvalue_2 "LockOnCapture"))

(fn LoadVictoryDeathMenu
  (bind _returnvalue (Game|GetPlayerController 0))
  (bind _returnvalue_2 (UserInterface|CreateWidget "/Game/UI/WBP_VictoryDeathMenu.WBP_VictoryDeathMenu_C" _returnvalue))
  (UserInterface|Viewport|AddtoViewport _returnvalue_2 0)
  (Input|SetInputModeUIOnly _returnvalue _returnvalue_2 "DoNotLock"))

(fn LoadEscapeMenu
  (bind _returnvalue (Game|GetPlayerController 0))
  (bind _returnvalue_2 (UserInterface|CreateWidget "/Game/UI/WBP_EscapeMenu.WBP_EscapeMenu_C" _returnvalue))
  (UserInterface|Viewport|AddtoViewport _returnvalue_2 0)
  (Input|SetInputModeUIOnly _returnvalue _returnvalue_2 "DoNotLock")
  (Variables|/Script/Engine.PlayerController|SetbShowMouseCursor _returnvalue true))

(fn InitializeMainMenu
  (bind _returnvalue (Game|GetPlayerController 0))
  (bind _returnvalue_2 (UserInterface|CreateWidget "/Game/UI/WBP_MainMenu.WBP_MainMenu_C" _returnvalue))
  (UserInterface|Viewport|AddtoViewport _returnvalue_2 0)
  (Input|SetInputModeUIOnly _returnvalue _returnvalue_2 "LockOnCapture")
  (Variables|/Script/Engine.PlayerController|SetbShowMouseCursor _returnvalue true))

(fn ResumeGame
  (bind _returnvalue (Game|GetPlayerController 0))
  (Input|SetInputModeGameOnly _returnvalue)
  (Variables|/Script/Engine.PlayerController|SetbShowMouseCursor _returnvalue false))