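; BP_ZombieCharacter is an enemy zombie that chases the player while the player is inside its detection sphere.
; Sphere overlaps set or clear the player reference, switch directly between looping run and idle animations, and stop movement when the player leaves.
; Tick reissues a simple move to the player's location while that reference is valid.
; The construction script randomly applies one of two skin textures through a dynamic material instance.
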(event OnComponentBeginOverlap(DetectionSphere)
  (params (OverlappedComponent :type Primitive%20Component%20Object%20Reference) (OtherActor :type Actor%20Object%20Reference) (OtherComp :type Primitive%20Component%20Object%20Reference) (OtherBodyIndex :type Integer) (bFromSweep :type Boolean) (SweepResult :type Hit%20Result%20Structure%20%28by%20ref%29))
  (bind _asbp_player_character (Utilities|Casting|CastToBP_PlayerCharacter OtherActor))
  (Variables|Default|SetPlayerCharacter _asbp_player_character)
  (CallFunction|ToggleAnimation true))

(event OnComponentEndOverlap(DetectionSphere)
  (params (OverlappedComponent :type Primitive%20Component%20Object%20Reference) (OtherActor :type Actor%20Object%20Reference) (OtherComp :type Primitive%20Component%20Object%20Reference) (OtherBodyIndex :type Integer))
  (bind _self self)
  (bind _asbp_player_character (Utilities|Casting|CastToBP_PlayerCharacter OtherActor))
  (if (== _asbp_player_character (Variables|Default|GetPlayerCharacter))
    (Variables|Default|SetPlayerCharacter 0)
    (CallFunction|ToggleAnimation false)
    (AI|Navigation|SimpleMovetoLocation (Pawn|GetController _self) (Transformation|GetActorLocation _self))))

(event EventBeginPlay
  (Components|Animation|PlayAnimation (Variables|Character|GetMesh) "/Game/Character/idle_Root_Idle.idle_Root_Idle" true))

(event EventTick
  (params (DeltaSeconds :type Float%20%28single-precision%29))
  (CallFunction|PursuePlayer))

(fn ConstructionScript
  (bind _returnvalue (Rendering|Material|CreateDynamicMaterialInstance (Variables|Character|GetMesh) 0 "/Game/Character/CharacterSkin_MI.CharacterSkin_MI" "None" :!class /Script/Engine.PrimitiveComponent))
  (Rendering|Material|SetTextureParameterValue _returnvalue "Skin" (Utilities|Array|Get(acopy) (Variables|Default|GetZombieSkins) (Math|Random|RandomInteger 2))))

(fn PursuePlayer
  (bind _playercharacter (Variables|Default|GetPlayerCharacter))
  (if (Utilities|IsValid _playercharacter)
    (AI|Navigation|SimpleMovetoLocation (Pawn|GetController self) (Transformation|GetActorLocation _playercharacter))))

(fn ToggleAnimation
  (params (IsMoving :type Boolean))
  (bind _mesh (Variables|Character|GetMesh))
  (if IsMoving
    (Components|Animation|PlayAnimation _mesh "/Game/Character/run_Root_Run.run_Root_Run" true)
    (else
      (Components|Animation|PlayAnimation _mesh "/Game/Character/idle_Root_Idle.idle_Root_Idle" true))))