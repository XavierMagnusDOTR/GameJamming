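; Player pawn with eight-direction WASD movement, idle and run animations, and a selectable skin.
; Key events set direction flags and toggle the looping animation.
; Each Tick snaps the collision component to a fixed world heading, offsets it along local X, and interpolates CameraElevation toward it for a loose follow camera.
; BeginPlay applies the game instance's skin index through a dynamic material's texture parameter.
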(event EventBeginPlay
  (bind _asbp_main_game_instance (Utilities|Casting|CastToBP_MainGameInstance (Game|GetGameInstance)))
  (CallFunction|SetCharacterSkin (Variables|/Game/BP_MainGameInstance.BP_MainGameInstance_C|GetCharacterSkin _asbp_main_game_instance)))

(event EventTick
  (params (DeltaSeconds :type Float%20%28single-precision%29))
  (CallFunction|CharacterRotation)
  (CallFunction|CharacterMovement DeltaSeconds)
  (CallFunction|LooseCameraFollow DeltaSeconds))

(event Input|KeyboardEvents|W
  (params (Key :type Key%20Structure :default "None"))
  (:Pressed
    (Variables|Default|SetIsPressedW true)
    (CallFunction|ToggleRunAnimation :!label _label))
  (:Released
    (Variables|Default|SetIsPressedW false)
    (goto _label)))

(event Input|KeyboardEvents|S
  (params (Key :type Key%20Structure :default "None"))
  (:Pressed
    (Variables|Default|SetIsPressedS true)
    (CallFunction|ToggleRunAnimation :!label _label))
  (:Released
    (Variables|Default|SetIsPressedS false)
    (goto _label)))

(event Input|KeyboardEvents|A
  (params (Key :type Key%20Structure :default "None"))
  (:Pressed
    (Variables|Default|SetIsPressedA true)
    (CallFunction|ToggleRunAnimation :!label _label))
  (:Released
    (Variables|Default|SetIsPressedA false)
    (goto _label)))

(event Input|KeyboardEvents|D
  (params (Key :type Key%20Structure :default "None"))
  (:Pressed
    (Variables|Default|SetIsPressedD true)
    (CallFunction|ToggleRunAnimation :!label _label))
  (:Released
    (Variables|Default|SetIsPressedD false)
    (goto _label)))

(fn ConstructionScript)

(fn CharacterRotation
  (bind _ispresseds (Variables|Default|GetIsPressedS))
  (bind _ispresseda (Variables|Default|GetIsPressedA))
  (bind _ispressedd (Variables|Default|GetIsPressedD))
  (bind _charactercollision (Variables|Default|GetCharacterCollision))
  (bind _charactercollision_2 (Variables|Default|GetCharacterCollision))
  (bind _ispressedw (Variables|Default|GetIsPressedW))
  (if (and _ispressedw _ispresseda)
    (Transformation|SetWorldRotation _charactercollision "0,315.000000, 0" false false)
    (elif (and _ispressedw _ispressedd)
      (Transformation|SetWorldRotation _charactercollision "0,45.000000, 0" false false)
      (elif (and _ispresseds _ispresseda)
        (Transformation|SetWorldRotation _charactercollision "0,225.000000, 0" false false)
        (elif (and _ispresseds _ispressedd)
          (Transformation|SetWorldRotation _charactercollision "0,135.000000, 0" false false)
          (elif (Variables|Default|GetIsPressedW)
            (Transformation|SetWorldRotation _charactercollision_2 "0, 0, 0" false false)
            (elif (Variables|Default|GetIsPressedS)
              (Transformation|SetWorldRotation _charactercollision_2 "0,180.000000, 0" false false)
              (elif (Variables|Default|GetIsPressedA)
                (Transformation|SetWorldRotation _charactercollision_2 "0,270.000000, 0" false false)
                (elif (Variables|Default|GetIsPressedD)
                  (Transformation|SetWorldRotation _charactercollision_2 "0,90.000000, 0" false false))))))))))

(fn LooseCameraFollow
  (params (InDelta :type Float%20%28single-precision%29))
  (bind _cameraelevation (Variables|Default|GetCameraElevation))
  (Transformation|SetWorldLocation _cameraelevation (Math|Interpolation|VInterpTo (Transformation|GetWorldLocation _cameraelevation) (Transformation|GetWorldLocation (Variables|Default|GetCharacterCollision)) InDelta 1e+01) false false))

(fn ToggleRunAnimation
  (bind _characterskelmesh (Variables|Default|GetCharacterSkelMesh))
  (if (Math|Boolean|ORBoolean (Variables|Default|GetIsPressedW) (Variables|Default|GetIsPressedS) (Variables|Default|GetIsPressedA) (Variables|Default|GetIsPressedD))
    (Components|Animation|PlayAnimation _characterskelmesh "/Game/Character/run_Root_Run.run_Root_Run" true)
    (else
      (Components|Animation|PlayAnimation _characterskelmesh "/Game/Character/idle_Root_Idle.idle_Root_Idle" true))))

(fn CharacterMovement
  (params (InDelta :type Float%20%28single-precision%29))
  (if (Math|Boolean|ORBoolean (Variables|Default|GetIsPressedW) (Variables|Default|GetIsPressedS) (Variables|Default|GetIsPressedA) (Variables|Default|GetIsPressedD))
    (Transformation|AddLocalOffset (Variables|Default|GetCharacterCollision) (Math|Vector|MakeVector (* InDelta 1e+03) 0.0 0.0) false false)))

(fn SetCharacterSkin
  (params (InIndex :type Integer))
  (bind _returnvalue (Rendering|Material|CreateDynamicMaterialInstance (Variables|Default|GetCharacterSkelMesh) 0 "/Game/Character/CharacterSkin_MI.CharacterSkin_MI" "None" :!class /Script/Engine.PrimitiveComponent))
  (Rendering|Material|SetTextureParameterValue _returnvalue "Skin" (Utilities|Array|Get(acopy) (Variables|Default|GetCharacterSkinArray) InIndex)))