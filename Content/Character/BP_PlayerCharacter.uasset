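; Player character for a zombie game, with eight-way WASD movement, a game-instance-selected skin and death or victory endings.
; Key flags snap the capsule's world yaw and drive forward movement each Tick, and toggle run/idle animations on key changes.
; The camera elevation component trails the capsule via VInterpTo.
; Zombie hits trigger death; each ending loads a game-instance menu, pauses and destroys the actor.
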(event OnComponentHit(CapsuleComponent)
  (params (HitComponent :type Primitive%20Component%20Object%20Reference) (OtherActor :type Actor%20Object%20Reference) (OtherComp :type Primitive%20Component%20Object%20Reference) (NormalImpulse :type Vector :default "0, 0, 0") (Hit :type Hit%20Result%20Structure%20%28by%20ref%29))
  (Utilities|Casting|CastToBP_ZombieCharacter OtherActor)
  (CallFunction|PlayerDeath "YOU WERE EATEN BY A ZOMBIE"))

(event EventBeginPlay
  (bind _asbp_main_game_instance (Utilities|Casting|CastToBP_MainGameInstance (Game|GetGameInstance)))
  (CallFunction|SetCharacterSkin (Variables|/Game/BP_MainGameInstance.BP_MainGameInstance_C|GetSkinID _asbp_main_game_instance)))

(event EventTick
  (params (DeltaSeconds :type Float%20%28single-precision%29))
  (CallFunction|LooseCameraFollow DeltaSeconds)
  (CallFunction|CharacterRotation)
  (CallFunction|ForwardMovement))

(event Input|KeyboardEvents|W
  (params (Key :type Key%20Structure))
  ;[1 1 1] Allows for diagonal movement if more than one key is pressed.
  (:Pressed
    (Variables|Default|SetIsPressedW true)
    (CallFunction|ToggleRunAnimation :!label _label))
  (:Released
    (Variables|Default|SetIsPressedW false)
    (goto _label)))

(event Input|KeyboardEvents|S
  (params (Key :type Key%20Structure))
  ;[1 1 1] Allows for diagonal movement if more than one key is pressed.
  (:Pressed
    (Variables|Default|SetIsPressedS true)
    (CallFunction|ToggleRunAnimation :!label _label))
  (:Released
    (Variables|Default|SetIsPressedS false)
    (goto _label)))

(event Input|KeyboardEvents|A
  (params (Key :type Key%20Structure))
  ;[1 1 1] Allows for diagonal movement if more than one key is pressed.
  (:Pressed
    (Variables|Default|SetIsPressedA true)
    (CallFunction|ToggleRunAnimation :!label _label))
  (:Released
    (Variables|Default|SetIsPressedA false)
    (goto _label)))

(event Input|KeyboardEvents|D
  (params (Key :type Key%20Structure))
  ;[1 1 1] Allows for diagonal movement if more than one key is pressed.
  (:Pressed
    (Variables|Default|SetIsPressedD true)
    (CallFunction|ToggleRunAnimation :!label _label))
  (:Released
    (Variables|Default|SetIsPressedD false)
    (goto _label)))

(fn ConstructionScript)

(fn ForwardMovement
  (if (Math|Boolean|ORBoolean (Variables|Default|GetIsPressedW) (Variables|Default|GetIsPressedS) (Variables|Default|GetIsPressedA) (Variables|Default|GetIsPressedD))
    (Pawn|Input|AddMovementInput (Math|Vector|GetForwardVector (Variables|Collision|GetCapsuleComponent)) 1.0 false)))

(fn LooseCameraFollow
  (params (InDelta :type Float%20%28single-precision%29))
  (bind _cameraelevation (Variables|Default|GetCameraElevation))
  (Transformation|SetWorldLocation _cameraelevation (Math|Interpolation|VInterpTo (Transformation|GetWorldLocation _cameraelevation) (Transformation|GetWorldLocation (Variables|Collision|GetCapsuleComponent)) InDelta 5.0) false false))

(fn CharacterRotation
  (bind _capsulecomponent (Variables|Collision|GetCapsuleComponent))
  (bind _capsulecomponent_2 (Variables|Collision|GetCapsuleComponent))
  (bind _ispresseds (Variables|Default|GetIsPressedS))
  (bind _ispresseda (Variables|Default|GetIsPressedA))
  (bind _ispressedd (Variables|Default|GetIsPressedD))
  (bind _ispressedw (Variables|Default|GetIsPressedW))
  (if (and _ispressedw _ispresseda)
    (Transformation|SetWorldRotation _capsulecomponent_2 "0,315.000000, 0" false false)
    (elif (and _ispressedw _ispressedd)
      (Transformation|SetWorldRotation _capsulecomponent_2 "0,45.000000, 0" false false)
      (elif (and _ispresseds _ispresseda)
        (Transformation|SetWorldRotation _capsulecomponent_2 "0,225.000000, 0" false false)
        (elif (and _ispresseds _ispressedd)
          (Transformation|SetWorldRotation _capsulecomponent_2 "0,135.000000, 0" false false)
          (elif (Variables|Default|GetIsPressedW)
            (Transformation|SetWorldRotation _capsulecomponent "0, 0, 0" false false)
            (elif (Variables|Default|GetIsPressedS)
              (Transformation|SetWorldRotation _capsulecomponent "0,180.000000, 0" false false)
              (elif (Variables|Default|GetIsPressedA)
                (Transformation|SetWorldRotation _capsulecomponent "0,270.000000, 0" false false)
                (elif (Variables|Default|GetIsPressedD)
                  (Transformation|SetWorldRotation _capsulecomponent "0,90.000000, 0" false false))))))))))

(fn ToggleRunAnimation
  (bind _mesh (Variables|Character|GetMesh))
  (if (Math|Boolean|ORBoolean (Variables|Default|GetIsPressedW) (Variables|Default|GetIsPressedS) (Variables|Default|GetIsPressedA) (Variables|Default|GetIsPressedD))
    (Components|Animation|PlayAnimation _mesh "/Game/Character/run_Root_Run.run_Root_Run" true)
    (else
      (Components|Animation|PlayAnimation _mesh "/Game/Character/idle_Root_Idle.idle_Root_Idle" true))))

(fn SetCharacterSkin
  (params (InIndex :type Integer))
  (bind _returnvalue (Rendering|Material|CreateDynamicMaterialInstance (Variables|Character|GetMesh) 0 "/Game/Character/CharacterSkin_MI.CharacterSkin_MI" "None" :!class /Script/Engine.PrimitiveComponent))
  (Rendering|Material|SetTextureParameterValue _returnvalue "Skin" (Utilities|Array|Get(acopy) (Variables|Default|GetCharacterSkinArray) InIndex)))

(fn PlayerDeath
  (params (InString :type String))
  (bind _asbp_main_game_instance (Utilities|Casting|CastToBP_MainGameInstance (Game|GetGameInstance)))
  (Default|LoadDeathMenu _asbp_main_game_instance InString)
  (Game|SetGamePaused true)
  (Actor|DestroyActor))

(fn PlayerFakeVictory
  (bind _asbp_main_game_instance (Utilities|Casting|CastToBP_MainGameInstance (Game|GetGameInstance)))
  (Default|LoadFakeVictoryMenu _asbp_main_game_instance)
  (Game|SetGamePaused true)
  (Actor|DestroyActor))

(fn PlayerVictory
  (bind _asbp_main_game_instance (Utilities|Casting|CastToBP_MainGameInstance (Game|GetGameInstance)))
  (Default|LoadVictoryMenu _asbp_main_game_instance)
  (Game|SetGamePaused true)
  (Actor|DestroyActor))