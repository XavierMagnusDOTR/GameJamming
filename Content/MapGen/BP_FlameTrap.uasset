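; Flame trap hazard in map generation that burns zombies and kills the player once triggered.
; A player entering the TriggerBox arms the trap and destroys zombies already inside the KillBox.
; While armed, anything entering the KillBox is killed, zombie or player.
; Tick runs a timer from activation that expires the trap after a fixed duration, disabling further kills on entry.
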(event OnComponentBeginOverlap(KillBox)
  (params (OverlappedComponent :type Primitive%20Component%20Object%20Reference) (OtherActor :type Actor%20Object%20Reference) (OtherComp :type Primitive%20Component%20Object%20Reference) (OtherBodyIndex :type Integer) (bFromSweep :type Boolean) (SweepResult :type Hit%20Result%20Structure%20%28by%20ref%29))
  (if (Variables|Default|GetIsTrapActive)
    (if (not (Variables|Default|GetIsTrapExpired))
      (bind _asbp_zombie_character (Utilities|Casting|CastToBP_ZombieCharacter OtherActor)
        (:then
          (Default|DestroyZombie _asbp_zombie_character))
        (:CastFailed
          (bind _asbp_player_character (Utilities|Casting|CastToBP_PlayerCharacter OtherActor))
          (Default|PlayerDeath _asbp_player_character "YOU BURNED UP IN A FLAME TRAP"))))))

(event OnComponentBeginOverlap(TriggerBox)
  (params (OverlappedComponent :type Primitive%20Component%20Object%20Reference) (OtherActor :type Actor%20Object%20Reference) (OtherComp :type Primitive%20Component%20Object%20Reference) (OtherBodyIndex :type Integer) (bFromSweep :type Boolean) (SweepResult :type Hit%20Result%20Structure%20%28by%20ref%29))
  (Utilities|Casting|CastToBP_PlayerCharacter OtherActor)
  (Variables|Default|SetIsTrapActive true)
  (CallFunction|KillOverlappingZombies))

(event EventTick
  (params (DeltaSeconds :type Float%20%28single-precision%29))
  (CallFunction|TrapTimerCountdown DeltaSeconds)
  (if (> (Variables|Default|GetTrapTimer) 15.0)
    (Variables|Default|SetIsTrapExpired true)))

(fn ConstructionScript)

(fn TrapTimerCountdown
  (params (InFloat :type Float%20%28single-precision%29))
  (if (Variables|Default|GetIsTrapActive)
    (Variables|Default|SetTrapTimer (+ (Variables|Default|GetTrapTimer) InFloat))))

(fn KillOverlappingZombies
  (for _array_element (Collision|GetOverlappingActors (Variables|Default|GetKillBox) "/Game/Character/BP_ZombieCharacter.BP_ZombieCharacter_C" :!class /Script/Engine.PrimitiveComponent)
    (bind _asbp_zombie_character (Utilities|Casting|CastToBP_ZombieCharacter _array_element))
    (Default|DestroyZombie _asbp_zombie_character)))