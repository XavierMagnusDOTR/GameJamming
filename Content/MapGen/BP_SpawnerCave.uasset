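; BP_SpawnerCave is a zombie spawner that activates when the player character enters its SpawnDetection volume, and nothing here deactivates it.
; While active, Tick accumulates a timer and spawns a BP_ZombieCharacter at the Spawner component after each NextSpawnDelay, up to a fixed lifetime cap.
; Each spawn attempt increments the local count and the shared ZombieCount on BP_MainGameInstance, even if collision blocks the spawn.
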(event OnComponentBeginOverlap(SpawnDetection)
  (params (OverlappedComponent :type Primitive%20Component%20Object%20Reference) (OtherActor :type Actor%20Object%20Reference) (OtherComp :type Primitive%20Component%20Object%20Reference) (OtherBodyIndex :type Integer) (bFromSweep :type Boolean) (SweepResult :type Hit%20Result%20Structure%20%28by%20ref%29))
  (Utilities|Casting|CastToBP_PlayerCharacter OtherActor)
  (Variables|Default|SetIsSpawnerActive true))

(event EventBeginPlay)

(event EventTick
  (params (DeltaSeconds :type Float%20%28single-precision%29))
  (if (Variables|Default|GetIsSpawnerActive)
    (bind _output_get (Variables|Default|SetNextSpawnTimer (+ DeltaSeconds (Variables|Default|GetNextSpawnTimer))))
    (if (> _output_get (Variables|Default|GetNextSpawnDelay))
      (Variables|Default|SetNextSpawnTimer 0.0)
      (if (not (>= (Variables|Default|GetAmountSpawned) 25))
        (Game|SpawnActorfromClass "/Game/Character/BP_ZombieCharacter.BP_ZombieCharacter_C" (Math|Transform|MakeTransform (Transformation|GetWorldLocation (Variables|Default|GetSpawner)) "0, 0, 0" "1,1,1") "AdjustIfPossibleButDontSpawnIfColliding" 0 0)
        (Math|Integer|IncrementInt (Variables|Default|GetAmountSpawned)
          (:%20%20
            (bind _asbp_main_game_instance (Utilities|Casting|CastToBP_MainGameInstance (Game|GetGameInstance)))
            (Math|Integer|IncrementInt (Variables|/Game/BP_MainGameInstance.BP_MainGameInstance_C|GetZombieCount _asbp_main_game_instance))))))))

(fn ConstructionScript)