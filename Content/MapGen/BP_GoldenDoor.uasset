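; BP_GoldenDoor is a map generation door that opens for the player and triggers a fake victory beyond a second overlap box.
; Player overlap with TriggerBox sets the open flag and disables door collision after a short delay.
; While open, Tick eases both door meshes downward with FInterpTo.
; DoorAttacked, not called here, accumulates attack time, then destroys the collision and opens the door.
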(event OnComponentBeginOverlap(TriggerBox)
  (params (OverlappedComponent :type Primitive%20Component%20Object%20Reference) (OtherActor :type Actor%20Object%20Reference) (OtherComp :type Primitive%20Component%20Object%20Reference) (OtherBodyIndex :type Integer) (bFromSweep :type Boolean) (SweepResult :type Hit%20Result%20Structure%20%28by%20ref%29))
  (Utilities|Casting|CastToBP_PlayerCharacter OtherActor)
  (Variables|Default|SetIsDoorOpen true)
  (CallFunction|DelayedDoorCollisionRemove))

(event OnComponentBeginOverlap(VictoryBox)
  (params (OverlappedComponent :type Primitive%20Component%20Object%20Reference) (OtherActor :type Actor%20Object%20Reference) (OtherComp :type Primitive%20Component%20Object%20Reference) (OtherBodyIndex :type Integer) (bFromSweep :type Boolean) (SweepResult :type Hit%20Result%20Structure%20%28by%20ref%29))
  (bind _asbp_player_character (Utilities|Casting|CastToBP_PlayerCharacter OtherActor))
  (Default|PlayerFakeVictory _asbp_player_character))

(event Custom|DelayedDoorCollisionRemove
  (Utilities|FlowControl|Delay 3.0)
  (Collision|SetCollisionEnabled (Variables|Default|GetDoorCollision) "NoCollision"))

(event EventTick
  (params (DeltaSeconds :type Float%20%28single-precision%29))
  (if (Variables|Default|GetIsDoorOpen)
    (CallFunction|DoorMovement DeltaSeconds)))

(fn ConstructionScript)

(fn DoorMovement
  (params (InDelta :type Float%20%28single-precision%29))
  (bind _goldendoorb (Variables|Default|GetGoldenDoorB))
  (bind _goldendoora (Variables|Default|GetGoldenDoorA))
  (bind _relativelocation (Variables|/Script/Engine.SceneComponent|GetRelativeLocation _goldendoora))
  (bind _relativelocation_2 (Variables|/Script/Engine.SceneComponent|GetRelativeLocation _goldendoorb))
  (Transformation|SetRelativeLocation _goldendoora (Math|Vector|MakeVector (.x _relativelocation) (.y _relativelocation) (Math|Interpolation|FInterpTo (.z _relativelocation) -4.7e+02 InDelta 1.0)) false false)
  (Transformation|SetRelativeLocation _goldendoorb (Math|Vector|MakeVector (.x _relativelocation_2) (.y _relativelocation_2) (Math|Interpolation|FInterpTo (.z _relativelocation_2) -2.6e+02 InDelta 1.0)) false false))

(fn DoorAttacked
  (params (InDelta :type Float%20%28single-precision%29))
  (bind _doorcollision (Variables|Default|GetDoorCollision))
  (if (> (Variables|Default|GetDoorAttackTimer) 1e+01)
    (if (Utilities|IsValid _doorcollision)
      (Components|DestroyComponent _doorcollision)
      (Variables|Default|SetIsDoorOpen true))
    (elif true
      (Variables|Default|SetDoorAttackTimer (+ InDelta (Variables|Default|GetDoorAttackTimer))))))