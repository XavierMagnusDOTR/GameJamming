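; BP_Doorway is a sliding double door that opens for the player and can be broken down by zombies.
; TriggerBox overlaps set the open and attacked flags and toggle DoorCollision for the player.
; Tick interpolates both panels toward open or closed positions and accumulates attack time while the attacked flag is set.
; Past the time threshold, the collision component is destroyed and the door stays open permanently; the timer never resets.
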(event OnComponentBeginOverlap(TriggerBox)
  (params (OverlappedComponent :type Primitive%20Component%20Object%20Reference) (OtherActor :type Actor%20Object%20Reference) (OtherComp :type Primitive%20Component%20Object%20Reference) (OtherBodyIndex :type Integer) (bFromSweep :type Boolean) (SweepResult :type Hit%20Result%20Structure%20%28by%20ref%29))
  (bind _doorcollision (Variables|Default|GetDoorCollision))
  (Utilities|Casting|CastToBP_PlayerCharacter OtherActor
    (:then
      (Variables|Default|SetIsDoorOpen true)
      (if (Utilities|IsValid _doorcollision)
        (Collision|SetCollisionEnabled _doorcollision "NoCollision")
        (Collision|SetCollisionResponsetoAllChannels _doorcollision "ECR_Ignore")))
    (:CastFailed
      (Utilities|Casting|CastToBP_ZombieCharacter OtherActor)
      (Variables|Default|SetIsDoorAttacked true))))

(event OnComponentEndOverlap(TriggerBox)
  (params (OverlappedComponent :type Primitive%20Component%20Object%20Reference) (OtherActor :type Actor%20Object%20Reference) (OtherComp :type Primitive%20Component%20Object%20Reference) (OtherBodyIndex :type Integer))
  (bind _doorcollision (Variables|Default|GetDoorCollision))
  (Utilities|Casting|CastToBP_PlayerCharacter OtherActor
    (:then
      (if (not (Variables|Default|GetIsDoorDestroyed))
        (Variables|Default|SetIsDoorOpen false)
        (if (Utilities|IsValid _doorcollision)
          (Collision|SetCollisionEnabled _doorcollision "QueryAndPhysics")
          (Collision|SetCollisionResponsetoAllChannels _doorcollision "ECR_Block"))))
    (:CastFailed
      (Utilities|Casting|CastToBP_ZombieCharacter OtherActor)
      (Variables|Default|SetIsDoorAttacked false))))

(event EventBeginPlay)

(event Collision|EventActorBeginOverlap
  (params (OtherActor :type Actor%20Object%20Reference)))

(event EventTick
  (params (DeltaSeconds :type Float%20%28single-precision%29))
  (CallFunction|DoorMovement DeltaSeconds)
  (CallFunction|DoorAttacked DeltaSeconds))

(fn ConstructionScript)

(fn DoorMovement
  (params (InDelta :type Float%20%28single-precision%29))
  (bind _doorleft (Variables|Default|GetDoorLeft))
  (bind _doorright (Variables|Default|GetDoorRight))
  (bind _doorleft_2 (Variables|Default|GetDoorLeft))
  (bind _doorright_2 (Variables|Default|GetDoorRight))
  (if (Variables|Default|GetIsDoorOpen)
    (Transformation|SetRelativeLocation _doorleft_2 (Math|Vector|MakeVector (Math|Interpolation|FInterpTo (.x (Variables|/Script/Engine.SceneComponent|GetRelativeLocation _doorleft_2)) -1.3e+02 InDelta 5.0) -4e+02 0.0) false false)
    (Transformation|SetRelativeLocation _doorright_2 (Math|Vector|MakeVector (Math|Interpolation|FInterpTo (.x (Variables|/Script/Engine.SceneComponent|GetRelativeLocation _doorright_2)) 1.3e+02 InDelta 5.0) -4e+02 0.0) false false)
    (else
      (Transformation|SetRelativeLocation _doorleft (Math|Vector|MakeVector (Math|Interpolation|FInterpTo (.x (Variables|/Script/Engine.SceneComponent|GetRelativeLocation _doorleft)) 0.0 InDelta 5.0) -4e+02 0.0) false false)
      (Transformation|SetRelativeLocation _doorright (Math|Vector|MakeVector (Math|Interpolation|FInterpTo (.x (Variables|/Script/Engine.SceneComponent|GetRelativeLocation _doorright)) 0.0 InDelta 5.0) -4e+02 0.0) false false))))

(fn DoorAttacked
  (params (InDelta :type Float%20%28single-precision%29))
  (bind _doorcollision (Variables|Default|GetDoorCollision))
  (if (> (Variables|Default|GetDoorAttackTimer) 1e+01)
    (if (Utilities|IsValid _doorcollision)
      (Components|DestroyComponent _doorcollision)
      (Variables|Default|SetIsDoorOpen true)
      (Variables|Default|SetIsDoorDestroyed true))
    (elif (Variables|Default|GetIsDoorAttacked)
      (Variables|Default|SetDoorAttackTimer (+ InDelta (Variables|Default|GetDoorAttackTimer))))))